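; BP_Element is an actor holding an element quantity, with a Plane and an EQ text display for the remaining amount.
; ElementReduction subtracts delta seconds from the quantity and updates the text, moving the actor to world origin once depleted.
; SetLocationAndRotation only fetches BP_MainCharacter actors, as its Plane and text placement nodes are disconnected.
; The event graph is empty, so neither function is called within this Blueprint.
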(event `self.ReceiveTick`
  (params (DeltaSeconds :type "Float (single-precision)")))

(fn `ElementReduction`
  (params (DeltaSeconds :type "Float (double-precision)"))
  (bind _elementquantity (`self.ElementQuantity`))
  (if (<= _elementquantity 0.0)
    (`self.K2_SetActorLocation` (0.0 0.0 0.0))
    (else
      (bind _output_get (set `self.ElementQuantity` (- _elementquantity DeltaSeconds)))
      (`TextRenderComponent.K2_SetText` (`self.EQ`) (`KismetTextLibrary.Conv_DoubleToText` _output_get "HalfToEven")))))

(fn `SetLocationAndRotation`
  (bind _outactors (`GameplayStatics.GetAllActorsOfClass` "/Game/Blueprints/BP_MainCharacter.BP_MainCharacter_C")))

(fn `UserConstructionScript`)